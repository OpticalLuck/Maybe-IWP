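; BP_Projectile_Shooter is an actor that automatically fires BP_Projectile instances at a repeating interval.
; One second after BeginPlay it starts the Shoot event, which re-calls itself after the Delay variable's interval, looping indefinitely.
; Each shot spawns a projectile at the Arrow component's location and sets its SphereMesh physics velocity along the arrow's forward vector, scaled by ShootForce.
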(event `self.ReceiveBeginPlay`
  (`KismetSystemLibrary.Delay` 1.0)
  (`self.Shoot`))

(event `Shoot`
  (bind _arrow (`self.Arrow`))
  (bind _returnvalue (`|SpawnActorFromClass` "/Game/2)Game/Blueprints/BP_Projectile.BP_Projectile_C" (`KismetMathLibrary.MakeTransform` (`SceneComponent.K2_GetComponentLocation` _arrow)) "Undefined" "OverrideRootScale" null null))
  (`PrimitiveComponent.SetPhysicsLinearVelocity` (`/Game/2)Game/Blueprints/BP_Projectile.SphereMesh` _returnvalue) (* (`SceneComponent.GetForwardVector` _arrow) (`self.Shoot Force`)) false "None")
  (`KismetSystemLibrary.Delay` (`self.Delay`))
  (`self.Shoot`))

(fn `UserConstructionScript`)