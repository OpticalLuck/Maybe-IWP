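; Parkour movement component that gives a Character side and vertical wall running, ledge grabs, mantling and jump-offs.
; A 60 Hz timer drives gated wall run, mantle and camera roll updates, with jump, land and movement-mode events toggling gates.
; Traces detect walls and ledges, LaunchCharacter propels runs, and interpolation completes mantles.
; A parkour mode enum tracks state, restoring gravity and movement mode on exit; timed gate reopening provides cooldowns.
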(event `Open WallRun Gate`
  (goto _label :!via `Open`))

(event `Close WallRun Gate`
  (goto _label :!via `Close`))

(event `PlayCameraShake`
  (params (CameraShake :type "MatineeCameraShake Class Reference"))
  (if (`self.CameraShake`)
    (`GameplayStatics.PlayWorldCameraShake` CameraShake (`Actor.K2_GetActorLocation` (`self.Character`)) 0.0 100.0)))

(event `Open Vertical WallRun Gate`
  (goto _label_2 :!via `Open`))

(event `Close Vertical WallRun Gate`
  (`self.Close Mantle Gate`)
  (goto _label_2 :!via `Close`))

(event `Open Mantle Check Gate`
  (goto _label_3 :!via `Open`))

(event `Close Mantle Check Gate`
  (goto _label_3 :!via `Close`))

(event `Open Mantle Gate`
  (goto _label_4 :!via `Open`))

(event `Close Mantle Gate`
  (goto _label_4 :!via `Close`))

(event `Mantle Check`
  (if (`self.CanMantle`)
    (`self.Mantle Start`)))

(event `Mantle Start`
  (bind _change (`self.Set ParkourMovementMode` "NewEnumerator5"))
  (if _change
    (`self.PlayCameraShake` (select `bool` (`self.QuickMantle`) :`false` "/Game/2)Game/Camera/Mantle.Mantle_C" :`true` "/Game/2)Game/Camera/QuickMantle.QuickMantle_C" :!type "MatineeCameraShake Class Reference"))
    (`self.Close Mantle Check Gate`)
    (`self.Open Mantle Gate`)))

(event `WallRun Update Event`
  (`|ExecutionSequence`
    (:`then_0`
      (`/Engine/EditorBlueprintResources/StandardMacros.Gate` true :!label _label
        (:`Exit`
          (`self.WallRun Update`))))
    (:`then_1`
      (`/Engine/EditorBlueprintResources/StandardMacros.Gate` true :!label _label_2
        (:`Exit`
          (`self.Vertical WallRun Update`))))
    (:`then_2`
      (`|ExecutionSequence`
        (:`then_0`
          (`/Engine/EditorBlueprintResources/StandardMacros.Gate` true :!label _label_3
            (:`Exit`
              (`self.Mantle Check`))))
        (:`then_1`
          (`/Engine/EditorBlueprintResources/StandardMacros.Gate` true :!label _label_4
            (:`Exit`
              (`self.Mantle Movement`))))))
    (:`then_3`
      (`self.Camera Tick`))))

(event `Initialize`
  (params (Character :type "Character Object Reference"))
  (bind _output_get (set `self.Character` Character))
  (bind _output_get_2 (set `self.Character Movement` (`Character.CharacterMovement` _output_get)))
  (set `self.Default Gravity` (`CharacterMovementComponent.GravityScale` _output_get_2))
  (`KismetSystemLibrary.K2_SetTimerDelegate` (delegate `WallRun Update Event`) 0.0167 true))

(event `Jump Event`
  (if (`|EnumEquality` (`self.Current Parkour Movement Mode`) "NewEnumerator0")
    (if (not (`NavMovementComponent.IsFalling` (`self.Character Movement`)))
      (`self.Open Gates`)
      (`self.PlayCameraShake` "/Game/2)Game/Camera/JumpLand.JumpLand_C"))
    (else
      (`self.Jump Events`))))

(event `Land Event`
  (`self.WallRun End` 0.0)
  (`self.Vertical WallRun End` 0.0)
  (`self.Close Gates`)
  (`self.PlayCameraShake` "/Game/2)Game/Camera/JumpLand.JumpLand_C"))

(event `MovementChanged`
  (params (`Prev Movement Mode` :type "EMovementMode Enum" :default "MOVE_None") (`New Movement Mode` :type "EMovementMode Enum" :default "MOVE_None"))
  (`/Engine/EditorBlueprintResources/StandardMacros.IsValid` (`self.Character Movement`)
    (:`Is Valid`
      (set `self.Prev Movement Mode` `Prev Movement Mode`)
      (set `self.Current Movement Mode` `New Movement Mode`)
      (if (and (`|EnumEquality` (`self.Prev Movement Mode`) "MOVE_Walking") (`|EnumEquality` (`self.Current Movement Mode`) "MOVE_Falling"))
        (`self.Open Gates`)))))

(event `ParkourMovementChanged`
  (params (`Prev Parkour Movement Mode` :type "/Game/2)Game/Enums/EParkourMovementMode Enum" :default "NewEnumerator0") (`New Parkour Movement Mode` :type "/Game/2)Game/Enums/EParkourMovementMode Enum" :default "NewEnumerator0"))
  (set `self.Prev Parkour Movement Mode` `Prev Parkour Movement Mode`)
  (set `self.Current Parkour Movement Mode` `New Parkour Movement Mode`)
  (`self.Reset Movement`))

(event `self.ReceiveTick`
  (params (DeltaSeconds :type "Float (single-precision)"))
  (`KismetSystemLibrary.PrintString` (`|GetEnumeratorNameAsString` (`self.Current Parkour Movement Mode`)) true true (struct :`G` 0.66 :`B` 1.0 :`A` 1.0) 0.0))

(fn `Camera Tick`
  (switch `/Game/2)Game/Enums/EParkourMovementMode` (`self.Current Parkour Movement Mode`)
    (:`NewEnumerator0`
      (`self.Camera Tilt` 0.0 :!label _label))
    (:`NewEnumerator1`
      (`self.Camera Tilt` 15.0))
    (:`NewEnumerator2`
      (`self.Camera Tilt` -15.0 :!label _label_2))
    (:`NewEnumerator3`
      (goto _label))
    (:`NewEnumerator4`
      (goto _label))
    (:`NewEnumerator5`
      (goto _label))
    (:`NewEnumerator6`
      (goto _label_2))
    (:`NewEnumerator7`
      (goto _label))))

(fn `Camera Tilt`
  (params (`Target X (Roll)` :type "Float (double-precision)"))
  (bind _returnvalue (`Controller.GetControlRotation` (`Pawn.GetController` (`self.Character`))))
  (`Controller.SetControlRotation` (`Pawn.GetController` (`self.Character`)) (`KismetMathLibrary.RInterpTo` _returnvalue (`KismetMathLibrary.MakeRotator` `Target X (Roll)` (.pitch _returnvalue) (.yaw _returnvalue)) (`GameplayStatics.GetWorldDeltaSeconds`) 10.0)))

(fn `Close Gates`
  (`self.Close WallRun Gate`)
  (`self.Close Vertical WallRun Gate`))

(fn `Jump Events`
  (`self.WallRun Jump`)
  (`self.LedgeGrab Jump`))

(fn `LedgeGrab Jump`
  (bind _current_parkour_movement_mode (`self.Current Parkour Movement Mode`))
  (bind (_vertical_wallrun_normal_x _vertical_wallrun_normal_y) (`KismetMathLibrary.BreakVector` (`self.Vertical WallRun Normal`)))
  (bind _ledge_jumpoff_force (`self.Ledge JumpOff Force`))
  (if (or (`|EnumEquality` _current_parkour_movement_mode "NewEnumerator4") (`|EnumEquality` _current_parkour_movement_mode "NewEnumerator3") (`|EnumEquality` _current_parkour_movement_mode "NewEnumerator5"))
    (`self.Vertical WallRun End` 0.35)
    (`Character.LaunchCharacter` (`self.Character`) (`KismetMathLibrary.MakeVector` (* _vertical_wallrun_normal_x _ledge_jumpoff_force) (* _ledge_jumpoff_force _vertical_wallrun_normal_y) (`self.Ledge Jump Height`)) false true)))

(fn `Mantle Movement`
  (bind _character (`self.Character`))
  (bind (_mantle_position_x _mantle_position_y) (`KismetMathLibrary.BreakVector` (`self.Mantle Position`)))
  (bind _character_2 (`self.Character`))
  (bind _returnvalue (`Pawn.GetController` _character))
  (bind (_returnvalue_x _returnvalue_y) (`KismetMathLibrary.BreakVector` (`Actor.K2_GetActorLocation` _character)))
  (`Controller.SetControlRotation` _returnvalue (`KismetMathLibrary.RInterpTo` (`Controller.GetControlRotation` _returnvalue) (`KismetMathLibrary.FindLookAtRotation` (`KismetMathLibrary.MakeVector` _returnvalue_x _returnvalue_y) (`KismetMathLibrary.MakeVector` _mantle_position_x _mantle_position_y)) (`GameplayStatics.GetWorldDeltaSeconds`) 7.0))
  (`Actor.K2_SetActorLocation` _character_2 (`KismetMathLibrary.VInterpTo` (`Actor.K2_GetActorLocation` _character_2) (`self.Mantle Position`) (`GameplayStatics.GetWorldDeltaSeconds`) (select `bool` (`self.QuickMantle`) :`false` (`self.Mantle Speed`) :`true` (`self.Quick Mantle Speed`))) false false)
  (if (< (`KismetMathLibrary.Vector_Distance` (`Actor.K2_GetActorLocation` (`self.Character`)) (`self.Mantle Position`)) 8.0)
    (`self.Vertical WallRun End` 0.5)))

(fn `Open Gates`
  (`self.Open WallRun Gate`)
  (`self.Open Vertical WallRun Gate`))

(fn `Reset Movement`
  (if (`|EnumEquality` (`self.Current Parkour Movement Mode`) "NewEnumerator0")
    (set `CharacterMovementComponent.GravityScale` (`self.Default Gravity`) (`self.Character Movement`))
    (`CharacterMovementComponent.SetMovementMode` (`self.Character Movement`) (select `/Game/2)Game/Enums/EParkourMovementMode` (`self.Prev Parkour Movement Mode`) :`NewEnumerator0` "MOVE_Falling" :`NewEnumerator1` "MOVE_Falling" :`NewEnumerator2` "MOVE_Falling" :`NewEnumerator3` "MOVE_Falling" :`NewEnumerator4` "MOVE_Falling" :`NewEnumerator5` "MOVE_Walking" :`NewEnumerator6` "MOVE_Walking" :`NewEnumerator7` "MOVE_Walking" :!type "EMovementMode Enum") 0)))

(fn `Set ParkourMovementMode`
  (params (`New ParkourMovement` :type "/Game/2)Game/Enums/EParkourMovementMode Enum" :default "NewEnumerator0"))
  (returns (Change :type Boolean))
  (bind _current_parkour_movement_mode (`self.Current Parkour Movement Mode`))
  (if (`|EnumEquality` `New ParkourMovement` _current_parkour_movement_mode)
    (return false)
    (else
      (`self.ParkourMovementChanged` _current_parkour_movement_mode (`local.New ParkourMovement`))
      (return true))))

(fn `Vertical WallRun End`
  (params (`Reset Time` :type "Float (double-precision)"))
  (bind _current_parkour_movement_mode (`self.Current Parkour Movement Mode`))
  (if (or (`|EnumEquality` _current_parkour_movement_mode "NewEnumerator5") (`|EnumEquality` _current_parkour_movement_mode "NewEnumerator4") (`|EnumEquality` _current_parkour_movement_mode "NewEnumerator3"))
    (bind _change (`self.Set ParkourMovementMode` "NewEnumerator0"))
    (if _change
      (`self.Close Vertical WallRun Gate`)
      (`self.Close Mantle Check Gate`)
      (`KismetSystemLibrary.K2_SetTimer` null "Open Vertical WallRun Gate" (`local.Reset Time`)))))

(fn `Vertical WallRun Movement`
  (bind (_eyes _feet) (`self.MantleVectors`))
  (bind (_returnvalue_x _returnvalue_y) (`KismetMathLibrary.BreakVector` (* (`self.Vertical WallRun Normal`) -600.0)))
  (bind (_outhit _returnvalue) (`KismetSystemLibrary.LineTraceSingle` _feet (+ _feet (* (`Actor.GetActorForwardVector` (`self.Character`)) 50.0)) "TraceTypeQuery1"))
  (if (and (> (`self.ForwardInput`) 0.0) _returnvalue)
    (set `self.Vertical WallRun Normal` (`.ImpactNormal` (`GameplayStatics.BreakHitResult` _outhit)))
    (`self.Set ParkourMovementMode` "NewEnumerator3")
    (`Character.LaunchCharacter` (`self.Character`) (`KismetMathLibrary.MakeVector` _returnvalue_x _returnvalue_y (`self.Vertical WallRun Speed`)) true true)
    (else
      (`self.Vertical WallRun End` 0.35))))

(fn `Vertical WallRun Update`
  (bind (_eyes _feet) (`self.MantleVectors`))
  (bind _character_movement (`self.Character Movement`))
  (if (`self.CanVerticalWallRun`)
    (bind (_outhit _returnvalue) (`KismetSystemLibrary.CapsuleTraceSingle` _eyes _feet 20.0 10.0 "TraceTypeQuery1"))
    (if _returnvalue
      (bind (_bblockinghit _binitialoverlap _time _distance _location _impactpoint) (`GameplayStatics.BreakHitResult` _outhit))
      (set `self.Mantle Trace Distance` _distance)
      (if (`CharacterMovementComponent.IsWalkable` (`self.Character Movement`) _outhit)
        (set `self.Mantle Position` (+ _impactpoint (`KismetMathLibrary.MakeVector` 0.0 0.0 (`CapsuleComponent.CapsuleHalfHeight` (`Character.CapsuleComponent` (`self.Character`))))))
        (`self.Close Vertical WallRun Gate`)
        (bind _change (`self.Set ParkourMovementMode` "NewEnumerator4"))
        (if _change
          (`CharacterMovementComponent.DisableMovement` _character_movement)
          (`MovementComponent.StopMovementImmediately` _character_movement)
          (set `CharacterMovementComponent.GravityScale` 0.0 _character_movement)
          (`self.PlayCameraShake` "/Game/2)Game/Camera/LedgeGrab.LedgeGrab_C")
          (if (`self.QuickMantle`)
            (`self.Open Mantle Check Gate`)
            (else
              (`KismetSystemLibrary.K2_SetTimer` null "Open Mantle Check Gate" 0.25))))
        (else
          (`self.Vertical WallRun Movement` :!label _label)))
      (else
        (goto _label)))
    (else
      (`self.Vertical WallRun End` 0.35))))

(fn `WallRun End`
  (params (`Reset Time` :type "Float (double-precision)"))
  (if (`self.IsWallRunning`)
    (`self.Set ParkourMovementMode` "NewEnumerator0")
    (`self.Close WallRun Gate`)
    (`KismetSystemLibrary.K2_SetTimer` null "Open WallRun Gate" (`local.Reset Time`))))

(fn `WallRun Jump`
  (bind _walljump_force (`self.WallJump Force`))
  (bind (_wallrun_normal_x _wallrun_normal_y) (`KismetMathLibrary.BreakVector` (`self.WallRun Normal`)))
  (if (`self.IsWallRunning`)
    (`self.WallRun End` (`self.WallJump Running Reset Timer`))
    (`Character.LaunchCharacter` (`self.Character`) (`KismetMathLibrary.MakeVector` (* _walljump_force _wallrun_normal_x) (* _walljump_force _wallrun_normal_y) (`self.WallJump Height`)) false true)))

(fn `WallRun Movement`
  (params (Start :type "Vector Structure") (End :type "Vector Structure") (`WallRun Direction` :type "Float (double-precision)"))
  (returns (Return :type Boolean))
  (bind _outhit (`KismetSystemLibrary.LineTraceSingle` Start End "TraceTypeQuery1"))
  (if (`GameplayStatics.BreakHitResult` _outhit)
    (bind (_returnvalue _out_vec2) (`self.Validate WallRun Vector` (`.Normal` (`GameplayStatics.BreakHitResult` _outhit))))
    (if (and (`NavMovementComponent.IsFalling` (`self.Character Movement`)) _returnvalue)
      (set `self.WallRun Normal` _out_vec2)
      (`Character.LaunchCharacter` (`self.Character`) (* (`KismetMathLibrary.Cross_VectorVector` (`self.WallRun Normal`) (0.0 0.0 1.0)) (* (`self.WallRun Speed`) (`local.WallRun Direction`))) true (not (`self.WallRun Gravity`))) ; Move Player Forward
      (return true)
      (else
        (return false)))
    (else
      (return false))))

(fn `WallRun Update`
  (if (`self.CanWallRun`)
    (bind _return (`self.WallRun Movement` (`Actor.K2_GetActorLocation` (`self.Character`)) (`self.WallRun End Vectors`) -1.0))
    (if _return
      (`self.Set ParkourMovementMode` "NewEnumerator2")
      (set `CharacterMovementComponent.GravityScale` (`KismetMathLibrary.FInterpTo` (`CharacterMovementComponent.GravityScale` (`self.Character Movement`)) (`self.WallRun Target Gravity`) (`GameplayStatics.GetWorldDeltaSeconds`) 10.0) (`self.Character Movement`))
      (elif (`|EnumEquality` (`self.Current Parkour Movement Mode`) "NewEnumerator2")
        (`self.WallRun End` (`self.WallRun Reset Timer`))
        (else
          (bind _return_2 (`self.WallRun Movement` (`Actor.K2_GetActorLocation` (`self.Character`)) (`.Left` (`self.WallRun End Vectors`)) 1.0))
          (if _return_2
            (`self.Set ParkourMovementMode` "NewEnumerator1")
            (set `CharacterMovementComponent.GravityScale` (`KismetMathLibrary.FInterpTo` (`CharacterMovementComponent.GravityScale` (`self.Character Movement`)) (`self.WallRun Target Gravity`) (`GameplayStatics.GetWorldDeltaSeconds`) 10.0) (`self.Character Movement`))
            (else
              (`self.WallRun End` (`self.WallRun Reset Timer`)))))))
    (else
      (`self.WallRun End` 1.0))))