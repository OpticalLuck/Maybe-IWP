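; Parkour movement Blueprint that gives an initialized Character wall running, wall jumping and camera tilt.
; A looping timer traces right, then left, and on a near-vertical wall while falling uses LaunchCharacter to stick and propel the character, easing gravity toward a target.
; Ending a run restores gravity and suppresses wall running on a timer, which landing clears.
; Tick rolls the control rotation according to the active wall side.
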(event `Reset WallRun Suppression`
  (`KismetSystemLibrary.K2_ClearTimer` null "Reset WallRun Suppression")
  (set `self.WallRun Suppressed` false))

(event `WallRun Update Event`
  (if (not (`self.WallRun Suppressed`))
    (`self.WallRun Update`)))

(event `Initialize`
  (params (Character :type "Character Object Reference"))
  (bind _output_get (set `self.Character` Character))
  (bind _output_get_2 (set `self.Character Movement` (`Character.CharacterMovement` _output_get)))
  (set `self.Default Gravity` (`CharacterMovementComponent.GravityScale` _output_get_2))
  (`KismetSystemLibrary.K2_SetTimerDelegate` (delegate `WallRun Update Event`) 0.2 true))

(event `self.ReceiveTick`
  (params (DeltaSeconds :type "Float (single-precision)"))
  (`self.Camera Tick`))

(event `Jump Event`
  (`self.WallRun Jump`))

(event `Land Event`
  (`self.WallRun End` 0.0)
  (set `self.WallRun Suppressed` false))

(fn `Camera Tick`
  (if (`self.WallRunningL`)
    (`self.Camera Tilt` 15.0)
    (elif (`self.WallRunningR`)
      (`self.Camera Tilt` -15.0)
      (else
        (`self.Camera Tilt` 0.0)))))

(fn `Camera Tilt`
  (params (`Target X (Roll)` :type "Float (double-precision)"))
  (bind _returnvalue (`Controller.GetControlRotation` (`Pawn.GetController` (`self.Character`))))
  (`Controller.SetControlRotation` (`Pawn.GetController` (`self.Character`)) (`KismetMathLibrary.RInterpTo` _returnvalue (`KismetMathLibrary.MakeRotator` `Target X (Roll)` (.pitch _returnvalue) (.yaw _returnvalue)) (`GameplayStatics.GetWorldDeltaSeconds`) 10.0)))

(fn `Suppress WallRun`
  (params (`Delay Timer` :type "Float (single-precision)"))
  (set `self.WallRun Suppressed` true)
  (`KismetSystemLibrary.K2_SetTimer` null "Reset WallRun Suppression" `Delay Timer`))

(fn `WallRun End`
  (params (`Reset Time` :type "Float (double-precision)"))
  (if (`self.WallRunning`)
    (set `self.WallRunning` false)
    (set `self.WallRunningL` false)
    (set `self.WallRunningR` false)
    (set `CharacterMovementComponent.GravityScale` (`self.Default Gravity`) (`self.Character Movement`))
    (`self.Suppress WallRun` (`local.Reset Time`))))

(fn `WallRun Jump`
  (bind _walljump_force (`self.WallJump Force`))
  (bind (_wallrun_normal_x _wallrun_normal_y) (`KismetMathLibrary.BreakVector` (`self.WallRun Normal`)))
  (if (`self.WallRunning`)
    (`self.WallRun End` (`self.WallJump Running Reset Timer`))
    (`Character.LaunchCharacter` (`self.Character`) (`KismetMathLibrary.MakeVector` (* _walljump_force _wallrun_normal_x) (* _walljump_force _wallrun_normal_y) (`self.WallJump Height`)) false true)))

(fn `WallRun Movement`
  (params (Start :type "Vector Structure") (End :type "Vector Structure") (`WallRun Direction` :type "Float (double-precision)"))
  (returns (Return :type Boolean))
  (bind _outhit (`KismetSystemLibrary.LineTraceSingle` Start End "TraceTypeQuery1"))
  (if (`GameplayStatics.BreakHitResult` _outhit)
    (bind (_returnvalue _out_vec2) (`self.Validate WallRun Vector` (`.Normal` (`GameplayStatics.BreakHitResult` _outhit))))
    (if (and (`NavMovementComponent.IsFalling` (`self.Character Movement`)) _returnvalue)
      (set `self.WallRun Normal` _out_vec2)
      (`Character.LaunchCharacter` (`self.Character`) (`self.Get PlayerToWall`) false false) ; Stick Player to Wall
      (`Character.LaunchCharacter` (`self.Character`) (* (`KismetMathLibrary.Cross_VectorVector` (`self.WallRun Normal`) (0.0 0.0 1.0)) (* (`self.WallRun Speed`) (`local.WallRun Direction`))) true (not (`self.WallRun Gravity`))) ; Move Player Forward
      (return true)
      (else
        (return false)))
    (else
      (return false))))

(fn `WallRun Update`
  (bind _return (`self.WallRun Movement` (`Actor.K2_GetActorLocation` (`self.Character`)) (`self.WallRun End Vectors`) -1.0))
  (if _return
    (bind _output_get (set `self.WallRunning` true))
    (set `self.WallRunningR` _output_get)
    (set `self.WallRunningL` false)
    (set `CharacterMovementComponent.GravityScale` (`KismetMathLibrary.FInterpTo` (`CharacterMovementComponent.GravityScale` (`self.Character Movement`)) (`self.WallRun Target Gravity`) (`GameplayStatics.GetWorldDeltaSeconds`) 10.0) (`self.Character Movement`))
    (elif (`self.WallRunningR`)
      (`self.WallRun End` (`self.WallRun Reset Timer`))
      (else
        (bind _return_2 (`self.WallRun Movement` (`Actor.K2_GetActorLocation` (`self.Character`)) (`.Left` (`self.WallRun End Vectors`)) 1.0))
        (if _return_2
          (bind _output_get_2 (set `self.WallRunning` true))
          (set `self.WallRunningL` _output_get_2)
          (set `self.WallRunningR` false)
          (set `CharacterMovementComponent.GravityScale` (`KismetMathLibrary.FInterpTo` (`CharacterMovementComponent.GravityScale` (`self.Character Movement`)) (`self.WallRun Target Gravity`) (`GameplayStatics.GetWorldDeltaSeconds`) 10.0) (`self.Character Movement`))
          (else
            (`self.WallRun End` (`self.WallRun Reset Timer`))))))))