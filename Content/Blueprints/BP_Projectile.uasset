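; BP_Projectile is a physics-driven projectile that damages any Character it hits and then destroys itself.
; On spawn it starts a despawn timer and makes its BP_Base_Character instigator's capsule ignore it when moving.
; Non-character hits destroy it unless CanBounce is set.
; Tick points the capsule's Z axis along its physics velocity; IsFriendly is set but only read in disconnected debug logic.
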(event `self.ReceiveBeginPlay`
  (`KismetSystemLibrary.K2_SetTimer` null "Despawn" (`self.Despawn Timer`))
  (bind _asbp_base_character (cast `/Game/Blueprints/Player/BP_Base_Character` (`self.GetInstigator`)))
  (`PrimitiveComponent.IgnoreActorWhenMoving` (`Character.CapsuleComponent` _asbp_base_character) self true)
  (set `self.IsFriendly` true))

(event `self.ReceiveHit`
  (params (MyComp :type "PrimitiveComponent Object Reference") (Other :type "Actor Object Reference") (OtherComp :type "PrimitiveComponent Object Reference") (bSelfMoved :type Boolean) (HitLocation :type "Vector Structure") (HitNormal :type "Vector Structure") (NormalImpulse :type "Vector Structure") (Hit :type "HitResult Structure (by ref)"))
  (bind _ascharacter (cast `Character` Other)
    (:`then`
      (`GameplayStatics.ApplyDamage` _ascharacter 20.0 (`self.GetInstigatorController`) self)
      (`self.Despawn`))
    (:`CastFailed`
      (if (not (`self.CanBounce`))
        (`self.Despawn`)))))

(event `Despawn`
  (`self.K2_DestroyActor`))

(event `self.ReceiveTick`
  (params (DeltaSeconds :type "Float (single-precision)"))
  (bind _returnvalue (`PrimitiveComponent.GetPhysicsLinearVelocity` (`self.Capsule`) "None"))
  (`SceneComponent.K2_SetWorldRotation` (`self.Capsule`) (`KismetMathLibrary.MakeRotFromZ` _returnvalue) false false))

(fn `UserConstructionScript`)