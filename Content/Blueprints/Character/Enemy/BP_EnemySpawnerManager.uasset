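; Enemy spawner manager that fills waves from the level's BP_EnemySpawner actors and tracks living enemies.
; The construction script gathers and takes ownership of the spawners; a bind event hooks it to the game manager's wave-start dispatcher.
; SpawnWave shuffles spawners, giving each a random share of remaining MaxEnemyCount, with the last taking the rest.
; Enemy removal increments the kill count and reports a clear once spawning is done and none remain.
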(event `BindGameManager`
  (params (GameManager :type "/Game/Blueprints/BP_GameManager Object Reference"))
  (bind _output_get (set `self.GameManager` GameManager))
  (add `/Game/Blueprints/BP_GameManager.ED_OnWaveStart` _output_get (`|CreateDelegate` :!event `SpawnWave`)))

(event `OnEnemyRemove`
  (params (Enemy :type "/Game/Blueprints/Character/Enemy/BP_Enemy_Character Object Reference"))
  (bind _enemylist (`self.EnemyList`))
  (`KismetArrayLibrary.Array_RemoveItem` _enemylist Enemy)
  (`/Engine/EditorBlueprintResources/StandardMacros.IncrementInt` (`/Game/Blueprints/BP_GameManager.EnemiesKilled` (`self.GameManager`))
    (:`  `
      (if (and (<= (`KismetArrayLibrary.Array_Length` _enemylist) 0) (`self.SpawnDone`))
        (`/Game/Blueprints/BP_GameManager.OnEnemyCleared` (`self.GameManager`))))))

(fn `SpawnWave`
  (locals (CurrentArrayElement :type "/Game/Blueprints/Character/Enemy/BP_EnemySpawner Object Reference"))
  (bind _spawnerlist (`self.SpawnerList`))
  (bind _returnvalue (- (`self.MaxEnemyCount`) (`KismetArrayLibrary.Array_Length` (`self.EnemyList`))))
  (set `self.SpawnDone` false)
  (`KismetArrayLibrary.Array_Shuffle` (`self.SpawnerList`))
  (for (_array_element _array_index) _spawnerlist
    (set `local.CurrentArrayElement` _array_element)
    (if (< (`KismetArrayLibrary.Array_Length` (`self.EnemyList`)) (`self.MaxEnemyCount`))
      (bind _enemyspawned (`/Game/Blueprints/Character/Enemy/BP_EnemySpawner.SpawnEnemies` (`local.CurrentArrayElement`) (`KismetMathLibrary.RandomIntegerInRange` (`KismetMathLibrary.SelectInt` _returnvalue 0 (`self.IsFinalIndex` _array_index _spawnerlist)) _returnvalue)))
      (`KismetArrayLibrary.Array_Append` (`self.EnemyList`) _enemyspawned)))
  (set `self.SpawnDone` true))

(fn `UserConstructionScript`
  (bind _outactors (`GameplayStatics.GetAllActorsOfClass` "/Game/Blueprints/Character/Enemy/BP_EnemySpawner.BP_EnemySpawner_C"))
  (bind _output_get (set `self.SpawnerList` _outactors))
  (for _array_element _output_get
    (`self.SetOwner` _array_element self)))