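; Enemy character Blueprint that spawns with a default weapon and is driven by a configurable default AI controller class.
; On BeginPlay it spawns the weapon, scales its projectile force by a velocity-reduction factor and adds it to its inventory.
; Guarded start/stop shooting events trigger item use, while a text render shows health every tick.
; Death awards cash to a killer with an inventory, and destruction notifies the enemy spawner manager.
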(event `self.ReceiveBeginPlay`
  (`parent.ReceiveBeginPlay`)
  (bind _returnvalue (`|SpawnActorFromClass` (`self.Default Weapon`) (`self.GetTransform`) "AlwaysSpawn" "OverrideRootScale" null null))
  (set `/Game/Blueprints/Items/Weapons/BP_Base_Weapon.Projectile Force` (* (`/Game/Blueprints/Items/Weapons/BP_Base_Weapon.Projectile Force` _returnvalue) (`self.VelocityReduction`)) _returnvalue)
  (`/Game/Blueprints/Component/BP_Inventory.Add To Inventory` (`self.BP_Inventory`) _returnvalue))

(event `self.OnPlayerDeath`
  (params (Causer :type "Actor Object Reference"))
  (bind _returnvalue (`self.GetComponentByClass` Causer "/Game/Blueprints/Component/BP_Inventory.BP_Inventory_C"))
  (`/Engine/EditorBlueprintResources/StandardMacros.IsValid` _returnvalue
    (:`Is Valid`
      (`/Game/Blueprints/Component/BP_Inventory.AddCash` _returnvalue 20)
      (`parent.OnPlayerDeath` Causer))))

(event `self.ReceiveDestroyed`
  (bind _returnvalue (`GameplayStatics.GetActorOfClass` "/Game/Blueprints/Character/Enemy/BP_EnemySpawnerManager.BP_EnemySpawnerManager_C"))
  (`/Engine/EditorBlueprintResources/StandardMacros.IsValid` _returnvalue
    (:`Is Valid`
      (`/Game/Blueprints/Character/Enemy/BP_EnemySpawnerManager.OnEnemyRemove` _returnvalue self))))

(event `self.ReceiveTick`
  (params (DeltaSeconds :type "Float (single-precision)"))
  (`TextRenderComponent.K2_SetText` (`self.TextRender`) (`KismetTextLibrary.Conv_DoubleToText` (`/Game/Blueprints/Component/BP_CharacterInfo.Health` (`self.BP_CharacterInfo`)) "HalfToEven")))

(event `StartShooting`
  (if (`self.CanShoot`)
    (if (not (`self.IsShooting`))
      (`self.On Item Use Pressed`)
      (set `self.IsShooting` true))))

(event `StopShooting`
  (if (`self.CanShoot`)
    (`self.On Item Use Released`)
    (set `self.IsShooting` false)))

(fn `UserConstructionScript`
  (`parent.UserConstructionScript`)
  (set `self.AIControllerClass` (`self.Default AI`)))