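; Base gameplay ability Blueprint that handles activation, an optional active duration and a cooldown, holding references to its owning character and ability component.
; Activation, gated by CanCast, runs the duration timer or completes immediately when there is none; completion then starts the cooldown, which restores CanCast.
; Tick feeds both timers through gates opened and closed by events, broadcasting normalized progress and completion through event dispatchers.
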(event `self.ReceiveBeginPlay`
  (add `self.ED_OnGAInitialized` (`|CreateDelegate` :!event `OnAbilityInitialized`)))

(event `/Game/Blueprints/Ability/BP_AbilityInterface.ActivateAbility`
  (if (`self.CanCast`)
    (set `self.CoolDown Timer` (`self.Base CoolDown`))
    (set `self.CanCast` false)
    (`/Game/Blueprints/Ability/BP_AbilityInterface.OnAbilityActivated`)
    (if (> (`self.Base Duration`) 0.0)
      (`self.Start Duration Timer`)
      (else
        (`/Game/Blueprints/Ability/BP_AbilityInterface.OnAbilityCompleted`)))))

(event `Stop Duration Timer`
  (goto _label :!via `Close`))

(event `Start Duration Timer`
  (set `self.Duration Timer` (`self.Base Duration`))
  (goto _label :!via `Open`))

(event `self.ReceiveTick`
  (params (DeltaSeconds :type "Float (single-precision)"))
  (`|ExecutionSequence`
    (:`then_0`
      (`/Engine/EditorBlueprintResources/StandardMacros.Gate` true :!label _label
        (:`Exit`
          (bind _done (`/Game/Blueprints/HelperFunctions.TimerFunction` (`self.Duration Timer`) DeltaSeconds))
          (if _done
            (`self.Stop Duration Timer`)
            (`/Game/Blueprints/Ability/BP_AbilityInterface.OnAbilityCompleted`)
            (`self.ED_AbilityCompleted`)
            (else
              (`self.ED_DurationTick` (/ (`self.Duration Timer`) (`self.Base Duration`))))))))
    (:`then_1`
      (`/Engine/EditorBlueprintResources/StandardMacros.Gate` true :!label _label_2
        (:`Exit`
          (bind _done_2 (`/Game/Blueprints/HelperFunctions.TimerFunction` (`self.CoolDown Timer`) DeltaSeconds))
          (if _done_2
            (set `self.CanCast` true)
            (`self.E_StopCoolDown`)
            (`self.ED_CoolDownCompleted`)
            (else
              (`self.ED_CoolDownTick` (/ (`self.CoolDown Timer`) (`self.Base CoolDown`))))))))))

(event `E_StartCoolDown`
  (goto _label_2 :!via `Open`))

(event `E_StopCoolDown`
  (goto _label_2 :!via `Close`))

(event `/Game/Blueprints/Ability/BP_AbilityInterface.OnAbilityCompleted`
  (`self.E_StartCoolDown`))

(fn `SetReferences`
  (params (Character :type "/Game/Blueprints/Character/BP_Base_Character Object Reference") (`Ability Component` :type "/Game/Blueprints/Component/BP_AbilityComponent Object Reference"))
  (set `self.Character Reference` Character)
  (set `self.Ability Component Reference` `Ability Component`)
  (`self.ED_OnGAInitialized`))