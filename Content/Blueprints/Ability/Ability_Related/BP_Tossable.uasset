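; BP_Tossable is a tossable ability actor that triggers a detonation on impact or on a timer.
; An overlap fires the detonate event when DetonateOnHit is set, and Tick fires it whenever TimerFunction on TimerExplosion returns true.
; The detonate event is empty here, so this file defines only the triggers.
; The construction script applies DefaultScale to the actor.
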(event `self.ReceiveActorBeginOverlap`
  (params (OtherActor :type "Actor Object Reference"))
  (if (`self.Detonate On Hit`)
    (`self.E OnExplosionDetonate`)))

(event `self.ReceiveTick`
  (params (DeltaSeconds :type "Float (single-precision)"))
  (bind _done (`/Game/Blueprints/HelperFunctions.TimerFunction` (`self.TimerExplosion`) DeltaSeconds))
  (if _done
    (`self.E OnExplosionDetonate`)))

(event `E OnExplosionDetonate`)

(fn `UserConstructionScript`
  (`self.SetActorScale3D` (`self.Default Scale`)))