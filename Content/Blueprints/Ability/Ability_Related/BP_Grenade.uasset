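; BP_Grenade is an explosive ability actor that detonates after a fuse or, optionally, on hitting anything other than its instigator.
; EActivateMechanism arms the fuse timer, which Tick evaluates through TimerFunction.
; Detonation applies full radial damage credited to the instigator's controller, fires a RadialForce impulse, draws a debug sphere and destroys the actor.
; The construction script sizes the RadialForce from the explosion radius and force settings.
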(event `self.E_ActivateMechanism`
  (set `self.Timer Detonate` (`self.Detonate Time`)))

(event `self.ReceiveHit`
  (params (MyComp :type "PrimitiveComponent Object Reference") (Other :type "Actor Object Reference") (OtherComp :type "PrimitiveComponent Object Reference") (bSelfMoved :type Boolean) (HitLocation :type "Vector Structure") (HitNormal :type "Vector Structure") (NormalImpulse :type "Vector Structure") (Hit :type "HitResult Structure (by ref)"))
  (if (and (`self.Detonate On Hit`) (!= (`self.Instigator`) Other))
    (`self.E OnExplosionDetonate`)))

(event `self.ReceiveTick`
  (params (DeltaSeconds :type "Float (single-precision)"))
  (bind _done (`/Game/Blueprints/HelperFunctions.TimerFunction` (`self.Timer Detonate`) DeltaSeconds))
  (if _done
    (`self.E OnExplosionDetonate`)))

(event `E OnExplosionDetonate`
  (`GameplayStatics.ApplyRadialDamage` :`BaseDamage` (`self.Explosion Damage`) :`Origin` (`self.K2_GetActorLocation`) :`DamageRadius` (`self.Explosion Radius`) :`DamageTypeClass` "/Script/Engine.DamageType" :`DamageCauser` self :`InstigatedByController` (`Pawn.GetController` (`self.GetInstigator`)) :`bDoFullDamage` true)
  (`RadialForceComponent.FireImpulse` (`self.RadialForce`))
  (`KismetSystemLibrary.DrawDebugSphere` (`self.K2_GetActorLocation`) (`self.Explosion Radius`) 32 (struct :`R` 1.0 :`G` 0.229848 :`A` 1.0) 1.0 2.0)
  (`self.K2_DestroyActor`))

(fn `UserConstructionScript`
  (bind _radialforce (`self.RadialForce`))
  (`parent.UserConstructionScript`)
  (set `RadialForceComponent.Radius` (`self.Explosion Radius`) _radialforce)
  (set `RadialForceComponent.ImpulseStrength` (`self.Explosion Force`) _radialforce))