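; GA_Impulse is an ability that fires a radial physics impulse from the owning character.
; On initialization it adds a RadialForceComponent to the character, configured from ImpulseStrength and ImpulseRadius as a constant-falloff velocity change that ignores the owner.
; Activation fires the impulse and briefly draws a debug sphere showing the affected radius.
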(event `/Game/Blueprints/Ability/BP_AbilityInterface.OnAbilityActivated`
  (bind _radial_force_component (`self.Radial Force Component`))
  (`RadialForceComponent.FireImpulse` _radial_force_component)
  (`KismetSystemLibrary.DrawDebugSphere` (`SceneComponent.K2_GetComponentLocation` _radial_force_component) (`self.Impulse Radius`) 12 (struct :`R` 1.0 :`G` 0.041269 :`A` 1.0) 3.0 1.0))

(event `/Game/Blueprints/Ability/BP_AbilityInterface.OnAbilityInitialized`
  (bind _radial_force_component (`self.Radial Force Component`))
  (bind _returnvalue (`|AddComponentByClass` :`self` (`self.Character Reference`) :`Class` "/Script/Engine.RadialForceComponent"))
  (set `self.Radial Force Component` _returnvalue)
  (set `RadialForceComponent.ImpulseStrength` (`self.Impulse Strength`) _radial_force_component)
  (set `RadialForceComponent.Radius` (`self.Impulse Radius`) _radial_force_component)
  (set `RadialForceComponent.bImpulseVelChange` true _radial_force_component)
  (set `RadialForceComponent.bIgnoreOwningActor` true _radial_force_component)
  (set `RadialForceComponent.Falloff` "RIF_Constant" _radial_force_component))