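; GA_TimeDilation is an ability that changes the flow of time for the world and its owning character while active.
; On activation it sets global time dilation, then sets the character's custom dilation to the self factor divided by the global one, so the character's effective speed is independent of the world's.
; On completion it calls the parent handler and restores both dilations to normal.
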(event `self.ReceiveTick`
  (params (DeltaSeconds :type "Float (single-precision)"))
  (`parent.ReceiveTick` DeltaSeconds))

(event `/Game/Blueprints/Ability/BP_AbilityInterface.OnAbilityActivated`
  (bind _globaldilationfactor (`self.GlobalDilationFactor`))
  (`GameplayStatics.SetGlobalTimeDilation` _globaldilationfactor)
  (set `Actor.CustomTimeDilation` (/ (`self.SelfDilationFactor`) _globaldilationfactor) (`self.Character Reference`)))

(event `/Game/Blueprints/Ability/BP_AbilityInterface.OnAbilityCompleted`
  (`parent.OnAbilityCompleted`)
  (`GameplayStatics.SetGlobalTimeDilation` 1.0)
  (set `Actor.CustomTimeDilation` 1.0 (`self.Character Reference`)))