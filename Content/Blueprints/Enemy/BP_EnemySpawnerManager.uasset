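; Enemy spawner manager that runs waves across the level's BP_EnemySpawner actors and tracks the spawned enemies.
; Its construction script gathers every spawner and sets itself as their owner.
; SpawnWave calls each spawner with a random integer and appends the returned enemies to EnemyList.
; OnEnemyRemove drops an enemy from that list and notifies GameManager through OnEnemyCleared once it is empty.
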(event `self.ReceiveBeginPlay`)

(event `OnEnemyRemove`
  (params (Enemy :type "/Game/Blueprints/Enemy/BP_Enemy_Character Object Reference"))
  (bind _enemylist (`self.EnemyList`))
  (`KismetArrayLibrary.Array_RemoveItem` _enemylist Enemy)
  (if (<= (`KismetArrayLibrary.Array_Length` _enemylist) 0)
    (`/Game/Blueprints/BP_GameManager.OnEnemyCleared` (`self.GameManager`))))

(fn `SpawnWave`
  (for _array_element (`self.SpawnerList`)
    (bind _enemyspawned (`/Game/Blueprints/Enemy/BP_EnemySpawner.SpawnEnemy` _array_element (`KismetMathLibrary.RandomIntegerInRange` 1)))
    (`KismetArrayLibrary.Array_Append` (`self.EnemyList`) _enemyspawned)))

(fn `UserConstructionScript`
  (bind _outactors (`GameplayStatics.GetAllActorsOfClass` "/Game/Blueprints/Enemy/BP_EnemySpawner.BP_EnemySpawner_C"))
  (bind _output_get (set `self.SpawnerList` _outactors))
  (for _array_element _output_get
    (`self.SetOwner` _array_element self)))