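; Enemy spawner Blueprint whose SpawnEnemy function spawns a requested count of SpawnTarget pawns and returns EnemyArr.
; Each uses the behavior tree from its DefaultAI class defaults, is cast to BP_Enemy_Character, linked via SpawnedFrom and stored.
; X/Y come from GetRandomPointInCollider, whose SpawnBox random-point node appears unconnected.
; Z adds the nearest overlapping actor's bounds half-height to the root's height.
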(event `self.ReceiveBeginPlay`)

(event `self.ReceiveTick`
  (params (DeltaSeconds :type "Float (single-precision)")))

(fn `SpawnEnemy`
  (params (count :type Integer))
  (returns (EnemySpawned :type "Array of /Game/Blueprints/Enemy/BP_Enemy_Character Object Reference"))
  (locals (EnemyArr :type "Array of /Game/Blueprints/Enemy/BP_Enemy_Character Object Reference"))
  (bind _returnvalue (`self.GetRandomPointInCollider`))
  (bind _spawntarget (`self.SpawnTarget`))
  (bind (_returnvalue_x _returnvalue_y _returnvalue_z) (`KismetMathLibrary.BreakVector` (`SceneComponent.K2_GetComponentLocation` (`self.DefaultSceneRoot`))))
  (for _ (range 1 (+ count 1))
    (bind _returnvalue_2 (`AIBlueprintHelperLibrary.SpawnAIFromClass` _spawntarget (defaults `Object` (`.Default AI` (defaults `Object` _spawntarget))) (`KismetMathLibrary.MakeVector` (.x _returnvalue) (.y _returnvalue) (+ _returnvalue_z (.z (`.BoxExtent` (`self.GetActorBounds` (`.ReturnValue` (`GameplayStatics.FindNearestActor` _returnvalue (`PrimitiveComponent.GetOverlappingActors` (`self.SpawnBox`) null))) true false))))) (struct) false self))
    (bind _asbp_enemy_character (cast `/Game/Blueprints/Enemy/BP_Enemy_Character` _returnvalue_2))
    (set `/Game/Blueprints/Enemy/BP_Enemy_Character.SpawnedFrom` self _asbp_enemy_character)
    (`KismetArrayLibrary.Array_Add` (`local.EnemyArr`) _asbp_enemy_character))
  (return (`local.EnemyArr`)))

(fn `UserConstructionScript`)