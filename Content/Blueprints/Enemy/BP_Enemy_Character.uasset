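; Enemy character Blueprint that fights with a spawned weapon and pays 20 cash to the killer's inventory when it dies.
; On BeginPlay it spawns its weapon class into its inventory, and construction assigns the default AI controller.
; Guarded start and stop shooting events press and release item use, while Tick shows current health on a text render.
; When destroyed, it notifies the enemy spawner manager of its removal.
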(event `self.OnPlayerDeath`
  (params (Causer :type "Actor Object Reference"))
  (`/Game/Blueprints/Component/BP_Inventory.AddCash` (`self.GetComponentByClass` Causer "/Game/Blueprints/Component/BP_Inventory.BP_Inventory_C") 20))

(event `self.ReceiveDestroyed`
  (bind _returnvalue (`GameplayStatics.GetActorOfClass` "/Game/Blueprints/Enemy/BP_EnemySpawnerManager.BP_EnemySpawnerManager_C"))
  (`/Engine/EditorBlueprintResources/StandardMacros.IsValid` _returnvalue
    (:`Is Valid`
      (`/Game/Blueprints/Enemy/BP_EnemySpawnerManager.OnEnemyRemove` _returnvalue self))))

(event `self.ReceiveBeginPlay`
  (`parent.ReceiveBeginPlay`)
  (bind _returnvalue (`|SpawnActorFromClass` (`self.Weapon`) (`self.GetTransform`) "AlwaysSpawn" "OverrideRootScale" null null))
  (`/Game/Blueprints/Component/BP_Inventory.Add To Inventory` (`self.BP_Inventory`) _returnvalue))

(event `self.ReceiveTick`
  (params (DeltaSeconds :type "Float (single-precision)"))
  (`TextRenderComponent.K2_SetText` (`self.TextRender`) (`KismetTextLibrary.Conv_DoubleToText` (`/Game/Blueprints/Component/BP_CharacteInfo.Health` (`self.BP_PlayerInfo`)) "HalfToEven")))

(event `StartShooting`
  (if (`self.CanShoot`)
    (if (not (`self.IsShooting`))
      (`self.On Item Use Pressed`)
      (set `self.IsShooting` true))))

(event `StopShooting`
  (if (`self.CanShoot`)
    (`self.On Item Use Released`)
    (set `self.IsShooting` false)))

(fn `UserConstructionScript`
  (`parent.UserConstructionScript`)
  (set `self.AIControllerClass` (`self.Default AI`)))