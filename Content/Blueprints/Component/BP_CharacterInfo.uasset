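; Character component that tracks health and armor for player and enemy characters and handles their death.
; Damage drains armor before spilling into health, then broadcasts remaining vitals; a bound UI component is initialized with this component.
; At zero health it disables the character once: players play a death montage, ragdoll and end the game through BP_GameManager.
; Enemies ragdoll, award cash to their killer and are destroyed by a Tick-driven despawn timer.
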(event `self.ReceiveTick`
  (params (DeltaSeconds :type "Float (single-precision)"))
  (bind _done (`/Game/Blueprints/HelperFunctions.TimerFunction` (`self.DespawnTimer`) DeltaSeconds))
  (if _done
    (`Actor.K2_DestroyActor` (`self.Character Ref`))))

(event `E_Damage Taken`
  (params (Damage :type "Float (double-precision)") (`Damage Type` :type "DamageType Object Reference") (`Instigated By` :type "Controller Object Reference") (`Damage Causer` :type "Actor Object Reference"))
  (if (!= self `Instigated By`)
    (`self.Take Damage` Damage)
    (if (== (`self.Health`) 0.0)
      (`self.E_OnHealthReachZero` (`Controller.K2_GetPawn` `Instigated By`)))))

(event `E_OnHealthReachZero`
  (params (Causer :type "Pawn Object Reference"))
  (bind _character_ref (`self.Character Ref`))
  (`/Engine/EditorBlueprintResources/StandardMacros.DoOnce` false
    (:`Completed`
      (`/Game/Blueprints/Character/BP_Base_Character.Disable Character` _character_ref)
      (if (`Pawn.IsPlayerControlled` _character_ref)
        (`self.E_OnPlayerDeath` Causer)
        (else
          (`self.E_OnEnemyDeath` Causer))))))

(event `E_OnPlayerDeath`
  (params (`Death Causer` :type "Pawn Object Reference"))
  (bind _character_ref (`self.Character Ref`))
  (`|PlayMontage` (`Character.Mesh` (`self.Character Ref`)) (`self.DeathMontage`)
    (:`then`
      (cast `/Game/Blueprints/Character/Player/BP_FirstPerson_FullBody_Character` _character_ref))
    (:`OnBlendOut`
      (`/Game/Blueprints/Character/BP_Base_Character.SetToRagdoll` _character_ref)
      (`KismetSystemLibrary.Delay` 1.0)
      (bind _returnvalue (`GameplayStatics.GetActorOfClass` "/Game/Blueprints/BP_GameManager.BP_GameManager_C"))
      (`/Game/Blueprints/BP_GameManager.EndGame` _returnvalue))))

(event `E_OnEnemyDeath`
  (params (`Death Causer` :type "Pawn Object Reference"))
  (bind _character_ref (`self.Character Ref`))
  (`|ExecutionSequence`
    (:`then_0`
      (`/Game/Blueprints/Character/BP_Base_Character.SetToRagdoll` _character_ref)
      (`PrimitiveComponent.AddImpulseAtLocation` (`Character.Mesh` _character_ref) (0.0 0.0 0.0) (0.0 0.0 0.0) "None")
      (set `self.DespawnTimer` (`self.TimeToDespawn`)))
    (:`then_1`
      (bind _asbp_enemy_character (cast `/Game/Blueprints/Character/Enemy/BP_Enemy_Character` (`self.Character Ref`)))
      (`/Game/Blueprints/Character/Enemy/BP_Enemy_Character.AddCashToDeathCauser` _asbp_enemy_character `Death Causer`))))

(fn `BindUIComponent`
  (params (UIComponent :type "/Game/Blueprints/Component/BP_UIComponent Object Reference"))
  (bind _output_get (set `self.UIComponent` UIComponent))
  (`/Game/Blueprints/Component/BP_UIComponent.InitializeCharacterInfo` _output_get self)
  (return))

(fn `GetCharacterVitals`
  (returns (Health :type "Float (double-precision)") (Armor :type "Float (double-precision)"))
  (return (`self.Health`) (`self.Armor`)))

(fn `Initialize`
  (params (Character :type "/Game/Blueprints/Character/BP_Base_Character Object Reference"))
  (set `self.Character Ref` Character)
  (bind _returnvalue (`GameplayStatics.GetActorOfClass` "/Game/Blueprints/BP_GameManager.BP_GameManager_C"))
  (add `self.ED_OnDeathAnimCompleted` (`|CreateDelegate` _returnvalue :!event `EndGame`))
  (return))

(fn `Take Damage`
  (params (Damage :type "Float (double-precision)"))
  (locals (`Remaining damage` :type "Float (double-precision)" :default 0.0))
  (bind (_health _armor) (`self.GetCharacterVitals`))
  (bind _armor_2 (`self.Armor`))
  (bind _damage (`local.Damage`))
  (`|ExecutionSequence`
    (:`then_0`
      (if (> (`self.Armor`) 0.0)
        (set `local.Remaining damage` (`KismetMathLibrary.FClamp` (- _damage _armor_2) 0.0 100.0))
        (set `self.Armor` (`KismetMathLibrary.FClamp` (- _armor_2 _damage) 0.0 100.0))
        (if (> (`local.Remaining damage`) 0.0)
          (set `self.Health` (`KismetMathLibrary.FClamp` (- (`self.Health`) (`local.Remaining damage`)) 0.0 100.0)))
        (else
          (set `self.Health` (`KismetMathLibrary.FClamp` (- (`self.Health`) (`local.Damage`)) 0.0 100.0)))))
    (:`then_1`
      (`self.ED_OnDamageTaken` _health _armor))))