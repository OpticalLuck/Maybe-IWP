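; Character info component that tracks health and armor for its owning character and handles damage and death.
; Player-controlled owners get a game UI widget at BeginPlay, updated as values change.
; Damage drains armor first, with any remainder reducing health.
; At zero health it disables the BP_Base_Character, stops AI logic and plays a death montage, destroying non-player characters when it completes.
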(event `self.ReceiveBeginPlay`
  (`self.Initialize UI`))

(event `Damage Taken`
  (params (Damage :type "Float (double-precision)") (`Damage Type` :type "DamageType Object Reference") (`Instigated By` :type "Actor Object Reference") (`Damage Causer` :type "Actor Object Reference"))
  (if (!= self `Instigated By`)
    (`self.Take Damage` Damage)
    (if (== (`self.Health`) 0.0)
      (`self.OnPlayerDeath`))))

(event `OnPlayerDeath`
  (bind _asbp_base_character (cast `/Game/Blueprints/Player/BP_Base_Character` (`self.GetOwner`)))
  (`/Game/Blueprints/Player/BP_Base_Character.DisableCharacter` _asbp_base_character)
  (if (not (`Pawn.IsPlayerControlled` _asbp_base_character))
    (`BrainComponent.StopLogic` (`AIController.BrainComponent` (`AIBlueprintHelperLibrary.GetAIController` _asbp_base_character)) ""))
  (`|PlayMontage` (`Character.Mesh` _asbp_base_character) "/Game/Assets/Characters/Mannequin_UE4/Animations/ThirdPersonAnims/Montage_Death.Montage_Death"
    (:`OnCompleted`
      (if (not (`Pawn.IsPlayerControlled` _asbp_base_character))
        (`Actor.K2_DestroyActor` _asbp_base_character)))))

(fn `Initialize UI`
  (bind _ascharacter (cast `Character` (`self.GetOwner`)))
  (if (`Pawn.IsPlayerControlled` _ascharacter)
    (bind _returnvalue (`|CreateWidget` "/Game/Blueprints/UI/BPUI_Game_UI.BPUI_Game_UI_C"))
    (bind _output_get (set `self.UI Reference` _returnvalue))
    (bind _ui (`/Game/Blueprints/UI/BPUI_Game_UI.Initialize` _output_get (`self.Health`) (`self.Armor`)))
    (`UserWidget.AddToViewport` _ui 0)))

(fn `Take Damage`
  (params (Damage :type "Float (double-precision)"))
  (locals (`Remaining damage` :type "Float (double-precision)" :default 0.0))
  (bind _armor (`self.Armor`))
  (bind _damage (`local.Damage`))
  (if (> (`self.Armor`) 0.0)
    (set `local.Remaining damage` (`KismetMathLibrary.FClamp` (- _damage _armor) 0.0 100.0))
    (bind _output_get (set `self.Armor` (`KismetMathLibrary.FClamp` (- _armor _damage) 0.0 100.0)))
    (bind _outputpin (`self.IsUIValid`)
      (:`Is Valid`
        (`/Game/Blueprints/UI/BPUI_Game_UI.Update Armor UI` _outputpin _output_get)
        (if (> (`local.Remaining damage`) 0.0)
          (bind _output_get_2 (set `self.Health` (`KismetMathLibrary.FClamp` (- (`self.Health`) (`local.Remaining damage`)) 0.0 100.0)))
          (bind _outputpin_2 (`self.IsUIValid`)
            (:`Is Valid`
              (`/Game/Blueprints/UI/BPUI_Game_UI.Update Health UI` _outputpin_2 _output_get_2))))))
    (else
      (bind _output_get_3 (set `self.Health` (`KismetMathLibrary.FClamp` (- (`self.Health`) (`local.Damage`)) 0.0 100.0)))
      (bind _outputpin_3 (`self.IsUIValid`)
        (:`Is Valid`
          (`/Game/Blueprints/UI/BPUI_Game_UI.Update Health UI` _outputpin_3 _output_get_3))))))