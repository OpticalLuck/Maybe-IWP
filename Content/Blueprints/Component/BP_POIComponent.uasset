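; BP_POIComponent is an actor component that registers its owner as a point of interest on the player's minimap.
; Shortly after BeginPlay, it reaches the minimap through Mode_Game, the BP_GameManager child actor and the player's UI component, then calls AddPOI with the owner and itself.
; It stores the returned widget and removes it from its parent on EndPlay.
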(event `self.ReceiveBeginPlay`
  (`KismetSystemLibrary.Delay` 0.2)
  (bind _asmode_game (cast `/Game/Blueprints/GameModes/Mode_Game` (`GameplayStatics.GetGameMode`)))
  (bind _asbp_game_manager (cast `/Game/Blueprints/BP_GameManager` (`ChildActorComponent.ChildActor` (`/Game/Blueprints/GameModes/Mode_Game.BP_GameManager` _asmode_game))))
  (bind _poi_widget (`/Game/Blueprints/UI/Minimap/BPUI_Minimap.Add POI` (`/Game/Blueprints/Component/BP_UIComponent.Minimap` (`/Game/Blueprints/Character/Player/BP_FirstPerson_FullBody_Character.BP_UIComponent` (`/Game/Blueprints/BP_GameManager.Player` _asbp_game_manager))) (`self.GetOwner`) self))
  (set `self.POI Widget` _poi_widget))

(event `self.ReceiveEndPlay`
  (params (EndPlayReason :type "EEndPlayReason Enum" :default "Destroyed"))
  (`Widget.RemoveFromParent` (`self.POI Widget`)))