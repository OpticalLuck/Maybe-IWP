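; Player info component for a Character that tracks health and armor and shows them in the game HUD.
; On BeginPlay it creates BPUI_Game_UI only if the owner is player-controlled, initializes it with both values and adds it to the viewport.
; DamageTaken drains armor first and carries any overflow into health, clamping results and pushing changes to the widget.
; UI updates use the widget reference without a validity check.
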(event `self.ReceiveBeginPlay`
  (`self.Initialize UI`))

(event `Damage Taken`
  (params (Damage :type "Float (double-precision)") (`Damage Type` :type "DamageType Object Reference") (`Instigated By` :type "Actor Object Reference") (`Damage Causer` :type "Actor Object Reference"))
  (`self.Take Damage` Damage))

(fn `Initialize UI`
  (bind _ascharacter (cast `Character` (`self.GetOwner`)))
  (if (`Pawn.IsPlayerControlled` _ascharacter)
    (bind _returnvalue (`|CreateWidget` "/Game/Blueprints/UI/BPUI_Game_UI.BPUI_Game_UI_C"))
    (bind _output_get (set `self.UI Reference` _returnvalue))
    (bind _ui (`/Game/Blueprints/UI/BPUI_Game_UI.Initialize` _output_get (`self.Health`) (`self.Armor`)))
    (`UserWidget.AddToViewport` _ui 0)))

(fn `Take Damage`
  (params (Damage :type "Float (double-precision)"))
  (locals (`Remaining damage` :type "Float (double-precision)" :default 0.0))
  (bind _armor (`self.Armor`))
  (bind _damage (`local.Damage`))
  (if (> (`self.Armor`) 0.0)
    (set `local.Remaining damage` (`KismetMathLibrary.FClamp` (- _damage _armor) 0.0 100.0))
    (bind _output_get (set `self.Armor` (`KismetMathLibrary.FClamp` (- _armor _damage) 0.0 100.0)))
    (`/Game/Blueprints/UI/BPUI_Game_UI.Update Armor UI` (`self.UI Reference`) _output_get)
    (if (> (`local.Remaining damage`) 0.0)
      (bind _output_get_2 (set `self.Health` (`KismetMathLibrary.FClamp` (- (`self.Health`) (`local.Remaining damage`)) 0.0 100.0)))
      (`/Game/Blueprints/UI/BPUI_Game_UI.Update Health UI` (`self.UI Reference`) _output_get_2))
    (else
      (bind _output_get_3 (set `self.Health` (`KismetMathLibrary.FClamp` (- (`self.Health`) (`local.Damage`)) 0.0 100.0)))
      (`/Game/Blueprints/UI/BPUI_Game_UI.Update Health UI` (`self.UI Reference`) _output_get_3))))