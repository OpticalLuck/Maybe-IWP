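; BP_UIComponent is a UI component that creates and holds the pause menu and in-game interface widgets for a player controller.
; On initialization it stores the supplied controller and creates both widgets with it as owning player, without adding either to the viewport here.
; It then binds the game interface to the BP_GameManager actor found in the world and fires OnGUIInitialized with that interface.
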(event `E_OnInitialize`
  (params (`Target Controller` :type "PlayerController Object Reference"))
  (bind _activecontroller (`self.ActiveController`))
  (set `self.ActiveController` `Target Controller`)
  (`|ExecutionSequence`
    (:`then_0`
      (bind _returnvalue (`|CreateWidget` "/Game/Blueprints/UI/BPUI_PauseMenu.BPUI_PauseMenu_C" _activecontroller))
      (set `self.PauseMenu` _returnvalue))
    (:`then_1`
      (bind _returnvalue_2 (`|CreateWidget` "/Game/Blueprints/UI/BPUI_Game_UI.BPUI_Game_UI_C" _activecontroller))
      (set `self.GameInterface` _returnvalue_2)
      (bind _returnvalue_3 (`GameplayStatics.GetActorOfClass` "/Game/Blueprints/BP_GameManager.BP_GameManager_C"))
      (`/Game/Blueprints/UI/BPUI_Game_UI.BindGameManager` (`self.GameInterface`) _returnvalue_3)
      (`self.OnGUIInitialized` (`self.GameInterface`)))))