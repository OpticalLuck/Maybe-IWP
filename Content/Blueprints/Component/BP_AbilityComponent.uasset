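; BP_AbilityComponent gives a character up to two abilities, a Movement one and a Combat one, triggered with Q and E.
; On initialization it caps the target class list at two, adds each class to the character as a component and stores it in a slot chosen by its AbilityType.
; The filled array goes to the UI component to build ability elements, and the key events activate abilities by slot index.
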(event `E_Initialize`
  (params (Character :type "/Game/Blueprints/Character/BP_Base_Character Object Reference") (UIComponent :type "/Game/Blueprints/Component/BP_UIComponent Object Reference"))
  (set `self.Character Ref` Character)
  (set `self.UI Component Ref` UIComponent)
  (`self.Resize Target Ability Class`)
  (for _array_element (`self.Target Ability Class`)
    (bind _returnvalue (`|AddComponentByClass` (`self.Character Ref`) _array_element))
    (`/Engine/EditorBlueprintResources/StandardMacros.IsValid` _returnvalue
      (:`Is Valid`
        (`KismetArrayLibrary.Array_Set` (`self.Abilities Array`) (select `/Game/Enums/EAbilityType` (`/Game/Blueprints/Ability/GA_Base.Ability Type` _returnvalue) :`NewEnumerator1` 1) _returnvalue))))
  (`/Game/Blueprints/Component/BP_UIComponent.InitializeAbilityUIElements` (`self.UI Component Ref`) (`self.Abilities Array`)))

(event `Key|Q`
  (params (Key :type "Key Structure"))
  (:`Pressed`
    (`/Game/Blueprints/Ability/GA_Base.ActivateAbility` (`|GetArrayItem` (`self.Abilities Array`)))))

(event `Key|E`
  (params (Key :type "Key Structure"))
  (:`Pressed`
    (`/Game/Blueprints/Ability/GA_Base.ActivateAbility` (`|GetArrayItem` (`self.Abilities Array`) 1))))