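; Base item Blueprint for pickups that add themselves to a BP_Base_Character's inventory on overlap.
; LinkToPlayer stores the character as owner reference and Instigator, attaches to its Weapon_R socket, updates item status and disables sphere collision.
; Equipping shows the item, enables tick and binds to the character's use-pressed and use-released events; unequipping reverses this.
; The item's use press and release events are empty stubs.
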(event `self.ReceiveActorBeginOverlap`
  (params (OtherActor :type "Actor Object Reference"))
  (bind _asbp_base_character (cast `/Game/Blueprints/Character/BP_Base_Character` OtherActor))
  (`/Game/Blueprints/Component/BP_Inventory.Add To Inventory` (`/Game/Blueprints/Character/BP_Base_Character.BP_Inventory` _asbp_base_character) self))

(event `OnItemUse Pressed`)

(event `OnItemUse Released`)

(event `Equip Item`
  (`self.SetActorHiddenInGame` (not true))
  (`self.SetActorTickEnabled` true)
  (`self.BindOnUseEvent`))

(event `UnEquip Item`
  (`self.SetActorHiddenInGame` (not false))
  (`self.SetActorTickEnabled` false)
  (`self.UnbindOnUseEvent`))

(fn `BindOnUseEvent`
  (bind _character_reference (`self.Character Reference`))
  (add `/Game/Blueprints/Character/BP_Base_Character.On Item Use Pressed` _character_reference (`|CreateDelegate` :!event `OnItemUse Pressed`))
  (add `/Game/Blueprints/Character/BP_Base_Character.On Item Use Released` _character_reference (`|CreateDelegate` :!event `OnItemUse Released`)))

(fn `Link To Player`
  (params (`Player Ref` :type "/Game/Blueprints/Character/BP_Base_Character Object Reference"))
  (bind _output_get (set `self.Character Reference` `Player Ref`))
  (set `self.Instigator` _output_get)
  (`self.K2_AttachToComponent` (`Character.Mesh` _output_get) "Weapon_R" "SnapToTarget" "SnapToTarget" "SnapToTarget")
  (set `self.Item Status` "NewEnumerator1")
  (`PrimitiveComponent.SetCollisionEnabled` (`self.Sphere`) "NoCollision")
  (set `self.IsPlayerControlled` (`Pawn.IsPlayerControlled` (`self.Character Reference`))))

(fn `UnbindOnUseEvent`
  (bind _character_reference (`self.Character Reference`))
  (remove `/Game/Blueprints/Character/BP_Base_Character.On Item Use Pressed` _character_reference (`|CreateDelegate` :!event `OnItemUse Pressed`))
  (remove `/Game/Blueprints/Character/BP_Base_Character.On Item Use Released` _character_reference (`|CreateDelegate` :!event `OnItemUse Released`)))

(fn `UserConstructionScript`)