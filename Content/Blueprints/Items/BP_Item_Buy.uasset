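; A purchasable item pickup that previews the item class set in ItemRef as a spinning, collision-disabled child actor with a price label.
; The label turns toward the camera on yaw and shows only within a set distance.
; Overlapping characters with a BP_PlayerInfo component get a crosshair tooltip naming the buy key.
; BuyItem spawns a fresh copy into the given inventory, while IsBuyable separately checks cash against Cost.
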(event `self.ReceiveBeginPlay`
  (bind _childactor (`self.ChildActor`))
  (`ActorComponent.Activate` _childactor false)
  (bind _asbp_base_item (cast `/Game/Blueprints/Items/BP_Base_Item` (`ChildActorComponent.ChildActor` _childactor)))
  (`PrimitiveComponent.SetCollisionEnabled` (`/Game/Blueprints/Items/BP_Base_Item.Sphere` _asbp_base_item) "NoCollision")
  (`TextRenderComponent.K2_SetText` (`self.TextRender`) (`|FormatText` "${Cost}" (`self.Cost`))))

(event `self.ReceiveTick`
  (params (DeltaSeconds :type "Float (single-precision)"))
  (`self.RotateChildAcor` DeltaSeconds)
  (`self.UpdateTextAnim`))

(event `self.ReceiveActorBeginOverlap`
  (params (OtherActor :type "Actor Object Reference"))
  (bind _asbp_base_character (cast `/Game/Blueprints/Player/BP_Base_Character` OtherActor))
  (bind _returnvalue (`self.GetComponentByClass` _asbp_base_character "/Game/Blueprints/Component/BP_PlayerInfo.BP_PlayerInfo_C"))
  (`/Engine/EditorBlueprintResources/StandardMacros.IsValid` _returnvalue
    (:`Is Valid`
      (`/Game/Blueprints/UI/BPUI_Game_UI.ToggleCrosshairToolTip` (`/Game/Blueprints/Component/BP_PlayerInfo.UI Reference` _returnvalue) true (`|FormatText` "Press [{KeyBinding}] to buy" (`KismetInputLibrary.Key_GetDisplayName` (`.Key` (break `InputActionKeyMapping` (`|GetArrayItem` (`InputSettings.GetActionMappingByName` (`InputSettings.GetInputSettings`) "Use/Buy"))))))))))

(event `self.ReceiveActorEndOverlap`
  (params (OtherActor :type "Actor Object Reference"))
  (bind _asbp_base_character (cast `/Game/Blueprints/Player/BP_Base_Character` OtherActor))
  (bind _returnvalue (`self.GetComponentByClass` _asbp_base_character "/Game/Blueprints/Component/BP_PlayerInfo.BP_PlayerInfo_C"))
  (`/Engine/EditorBlueprintResources/StandardMacros.IsValid` _returnvalue
    (:`Is Valid`
      (`/Game/Blueprints/UI/BPUI_Game_UI.ToggleCrosshairToolTip` (`/Game/Blueprints/Component/BP_PlayerInfo.UI Reference` _returnvalue) false (`|FormatText` "")))))

(fn `BuyItem`
  (params (Inventory :type "/Game/Blueprints/Component/BP_Inventory Object Reference"))
  (bind _returnvalue (`|SpawnActorFromClass` (`self.Item Ref`) (`KismetMathLibrary.MakeTransform` (0.0 0.0 -1000.0)) "AlwaysSpawn" "OverrideRootScale" null null))
  (`/Game/Blueprints/Component/BP_Inventory.Add To Inventory` Inventory _returnvalue))

(fn `IsBuyable`
  (params (InCash :type Integer))
  (returns (Buyable :type Boolean))
  (return (>= InCash (`self.Cost`))))

(fn `UserConstructionScript`
  (`ChildActorComponent.SetChildActorClass` (`self.ChildActor`) (`self.Item Ref`)))