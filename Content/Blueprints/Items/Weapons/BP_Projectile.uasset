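; Base gun projectile that reports character hits to the shooter's inventory component and despawns on a timer or on impact.
; Hits on the shooter are ignored, and bouncing projectiles or same-class collisions survive non-character impacts.
; Tick aligns the capsule's Z axis to its physics velocity and destroys the projectile if its instigator becomes invalid.
; SetCollisionChannel swaps block and overlap on two custom channels by friendliness.
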(event `self.ReceiveBeginPlay`
  (`KismetSystemLibrary.K2_SetTimerDelegate` (`|CreateDelegate` :!event `Despawn`) (`self.Despawn Timer`)))

(event `Despawn`
  (`self.K2_DestroyActor`))

(event `self.ReceiveHit`
  (params (MyComp :type "PrimitiveComponent Object Reference") (Other :type "Actor Object Reference") (OtherComp :type "PrimitiveComponent Object Reference") (bSelfMoved :type Boolean) (HitLocation :type "Vector Structure") (HitNormal :type "Vector Structure") (NormalImpulse :type "Vector Structure") (Hit :type "HitResult Structure (by ref)"))
  (if (!= (`self.CharacterRef`) Other)
    (bind _asbp_base_character (cast `/Game/Blueprints/Character/BP_Base_Character` Other)
      (:`then`
        (`/Game/Blueprints/Component/BP_Inventory.OnGunProjectileHit` (`self.GetComponentByClass` (`self.CharacterRef`) "/Game/Blueprints/Component/BP_Inventory.BP_Inventory_C") _asbp_base_character OtherComp (`self.WeaponRef`) self)
        (`self.Despawn`))
      (:`CastFailed`
        (if (and (!= (`GameplayStatics.GetObjectClass` Other) (`GameplayStatics.GetObjectClass` self)) (not (`self.CanBounce`)))
          (`self.Despawn`))))))

(event `self.ReceiveTick`
  (params (DeltaSeconds :type "Float (single-precision)"))
  (`/Engine/EditorBlueprintResources/StandardMacros.IsValid` (`self.GetInstigator`)
    (:`Is Valid`
      (bind _returnvalue (`PrimitiveComponent.GetPhysicsLinearVelocity` (`self.Collision Capsule`) "None"))
      (if (> (`KismetMathLibrary.VSizeSquared` _returnvalue) 0.0)
        (`SceneComponent.K2_SetWorldRotation` (`self.Collision Capsule`) (`KismetMathLibrary.MakeRotFromZ` _returnvalue) false true)))
    (:`Is Not Valid`
      (`self.Despawn`))))

(fn `SetCollisionChannel`
  (params (IsFriendly :type Boolean))
  (bind _returnvalue (enumliteral `ECollisionResponse` "ECR_Overlap"))
  (bind _returnvalue_2 (enumliteral `ECollisionResponse` "ECR_Block"))
  (bind _collision_capsule (`self.Collision Capsule`))
  (bind _isfriendly (`local.IsFriendly`))
  (`PrimitiveComponent.SetCollisionResponseToChannel` _collision_capsule "ECC_GameTraceChannel2" (select `bool` _isfriendly :`false` _returnvalue_2 :`true` _returnvalue))
  (`PrimitiveComponent.SetCollisionResponseToChannel` _collision_capsule "ECC_GameTraceChannel3" (select `bool` _isfriendly :`false` _returnvalue :`true` _returnvalue_2)))

(fn `SetReferences`
  (params (Character :type "/Game/Blueprints/Character/BP_Base_Character Object Reference") (Weapon :type "/Game/Blueprints/Items/Weapons/BP_Base_Weapon Object Reference"))
  (set `self.CharacterRef` Character)
  (set `self.WeaponRef` Weapon))

(fn `UserConstructionScript`
  (`self.SetActorScale3D` (`self.DefaultScale`)))