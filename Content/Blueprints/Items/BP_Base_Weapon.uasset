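; Base weapon item that fires hitscan shots while use is held, in semi-auto or automatic mode.
; A Tick gate queues each shot on a timer derived from RateOfFire, so even the first shot is delayed.
; Semi-auto keeps the queue flag set after firing until release clears it.
; FireGun line-traces from player 0's view point, currently only drawing the trace and printing the hit actor, without damage.
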(event `self.ReceiveTick`
  (params (DeltaSeconds :type "Float (single-precision)"))
  (`|ExecutionSequence`
    (:`then_0`
      (`/Engine/EditorBlueprintResources/StandardMacros.Gate` true :!label _label
        (:`Exit`
          (`self.QueueFireGun` (delegate `Is Firing`)))))))

(event `self.OnItemUse Pressed`
  (goto _label :!via `Open`))

(event `self.OnItemUse Released`
  (set `self.IsfireQueued` false)
  (goto _label :!via `Close`))

(event `Is Firing`
  (`self.FireGun`)
  (set `self.IsfireQueued` (`self.IsSemiAuto`)))

(fn `FireGun`
  (bind (_outlocation _outrotation) (`self.GetActorEyesViewPoint` (`GameplayStatics.GetPlayerPawn` 0)))
  (bind _outhit (`KismetSystemLibrary.LineTraceSingle` :`Start` _outlocation :`End` (+ _outlocation (* (`KismetMathLibrary.GetForwardVector` _outrotation) (`self.RayCase Distance`))) :`TraceChannel` "TraceTypeQuery1" :`DrawDebugType` "Persistent"))
  (`KismetSystemLibrary.PrintString` (`KismetSystemLibrary.GetDisplayName` (`.HitActor` (`GameplayStatics.BreakHitResult` _outhit))) true false (struct :`G` 0.66 :`B` 1.0 :`A` 1.0) 0.0))

(fn `QueueFireGun`
  (params (Delegate :type "Object Object Reference"))
  (if (not (`self.IsfireQueued`))
    (set `self.IsfireQueued` true)
    (`KismetSystemLibrary.K2_SetTimerDelegate` Delegate (/ 60.0 (`self.RateOfFire`)))))

(fn `UserConstructionScript`)