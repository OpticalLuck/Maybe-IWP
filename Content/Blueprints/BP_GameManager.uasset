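; BP_GameManager runs the countdown between enemy waves and tracks the wave count.
; Clearing enemies starts the timer and opens a gate that lets Tick decrement it; at zero it resets, increments the wave and closes the gate.
; Event dispatchers announce countdown start, countdown end and wave start.
; The construction script caches the player character and child-actor EnemySpawnerManager, giving the spawner a back-reference to this manager.
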(event `self.ReceiveBeginPlay`
  (`KismetSystemLibrary.K2_SetTimerDelegate` (`|CreateDelegate` :!event `OnCountDownStart`) 0.5))

(event `OnCountDownEnd`
  (`self.CountDownEnd`)
  (goto _label :!via `Close`))

(event `OnCountDownStart`
  (`self.StartTimer`)
  (goto _label :!via `Open`))

(event `OnCountDownTick`
  (params (Delta :type "Float (double-precision)"))
  (if (`self.CountingDown`)
    (set `self.CountDown Timer` (- (`self.CountDown Timer`) Delta))))

(event `self.ReceiveTick`
  (params (DeltaSeconds :type "Float (single-precision)"))
  (`/Engine/EditorBlueprintResources/StandardMacros.Gate` true :!label _label
    (:`Exit`
      (`|ExecutionSequence`
        (:`then_0`
          (`self.OnCountDownTick` DeltaSeconds))
        (:`then_1`
          (if (<= (`self.CountDown Timer`) 0.0)
            (`self.OnCountDownEnd`)))))))

(event `OnEnemyCleared`
  (`self.OnCountDownStart`))

(fn `GetCountDownMax`
  (returns (MaxCountdown :type "Float (double-precision)"))
  (return (`self.MaxCountdown`)))

(fn `GetCurrentCountDownTimer`
  (returns (`CountDown Timer` :type "Float (double-precision)"))
  (return (`self.CountDown Timer`)))

(fn `UserConstructionScript`
  (bind _returnvalue (`GameplayStatics.GetActorOfClass` "/Script/Engine.PlayerController"))
  (bind _asbp_base_character (cast `/Game/Blueprints/Character/BP_Base_Character` (`Controller.K2_GetPawn` _returnvalue)))
  (set `self.Player` _asbp_base_character)
  (bind _asbp_enemy_spawner_manager (cast `/Game/Blueprints/Character/Enemy/BP_EnemySpawnerManager` (`ChildActorComponent.ChildActor` (`self.BP_EnemySpawnerManager`))))
  (bind _output_get (set `self.EnemySpawnerManager` _asbp_enemy_spawner_manager))
  (set `/Game/Blueprints/Character/Enemy/BP_EnemySpawnerManager.GameManager` self _output_get))