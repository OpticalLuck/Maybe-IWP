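; Interactable checkout point that lets the player finish the game once their inventory holds enough cash.
; On BeginPlay it caches BP_GameManager and builds a tooltip showing the cash requirement.
; Player enter and exit events set or clear that tooltip through the character's BP_UIComponent.
; Invoking it compares inventory cash to the requirement and currently only prints a debug string on success.
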(event `self.ReceiveBeginPlay`
  (bind _returnvalue (`GameplayStatics.GetActorOfClass` "/Game/Blueprints/BP_GameManager.BP_GameManager_C"))
  (set `self.GameManager` _returnvalue)
  (set `self.ToolTipText` (`|FormatText` "Finish Game (requires ${amt})" (`self.CashRequirement`))))

(event `self.E OnPlayerEnter`
  (params (Character :type "/Game/Blueprints/Character/BP_Base_Character Object Reference"))
  (bind _returnvalue (`self.GetComponentByClass` Character "/Game/Blueprints/Component/BP_UIComponent.BP_UIComponent_C"))
  (`/Engine/EditorBlueprintResources/StandardMacros.IsValid` _returnvalue
    (:`Is Valid`
      (`/Game/Blueprints/Component/BP_UIComponent.ToggleToolTip` _returnvalue true (`/Game/Blueprints/HelperFunctions.GetInteractToolTipText` (`KismetTextLibrary.Conv_TextToString` (`self.ToolTipText`)))))))

(event `self.E OnPlayerExit`
  (params (Character :type "/Game/Blueprints/Character/BP_Base_Character Object Reference"))
  (bind _returnvalue (`self.GetComponentByClass` Character "/Game/Blueprints/Component/BP_UIComponent.BP_UIComponent_C"))
  (`/Engine/EditorBlueprintResources/StandardMacros.IsValid` _returnvalue
    (:`Is Valid`
      (`/Game/Blueprints/Component/BP_UIComponent.ToggleToolTip` _returnvalue true ""))))

(event `self.E Invoke`
  (params (Character :type "/Game/Blueprints/Character/BP_Base_Character Object Reference") (Inventory :type "/Game/Blueprints/Component/BP_Inventory Object Reference"))
  (if (>= (`/Game/Blueprints/Component/BP_Inventory.Cash` Inventory) (`self.CashRequirement`))
    (`KismetSystemLibrary.PrintString` "GGEZ")))

(fn `UserConstructionScript`)