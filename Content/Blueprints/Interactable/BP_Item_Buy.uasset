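; Interactable shop pickup that displays a spinning preview of an item with a price label and sells it to the player for cash.
; The construction script sets ItemRef on a child actor, whose item collision is disabled at play.
; Player enter and exit toggle a buy tooltip, and the price text faces the camera when in range.
; On interact with enough cash, it spawns a fresh item below the world, adds it to inventory and deducts the cost.
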(event `self.ReceiveBeginPlay`
  (bind _childactor (`self.ChildActor`))
  (`ActorComponent.Activate` _childactor true)
  (bind _asbp_base_item (cast `/Game/Blueprints/Items/BP_Base_Item` (`ChildActorComponent.ChildActor` _childactor)))
  (`PrimitiveComponent.SetCollisionEnabled` (`/Game/Blueprints/Items/BP_Base_Item.Sphere` _asbp_base_item) "NoCollision")
  (`TextRenderComponent.K2_SetText` (`self.TextRender`) (`|FormatText` "${Cost}" (`self.Cost`))))

(event `self.ReceiveTick`
  (params (DeltaSeconds :type "Float (single-precision)"))
  (`self.RotateChildAcor` DeltaSeconds)
  (`self.UpdateTextAnim`))

(event `self.E OnPlayerEnter`
  (params (Character :type "/Game/Blueprints/Character/BP_Base_Character Object Reference"))
  (bind _returnvalue (`self.GetComponentByClass` Character "/Game/Blueprints/Component/BP_UIComponent.BP_UIComponent_C"))
  (`/Engine/EditorBlueprintResources/StandardMacros.IsValid` _returnvalue
    (:`Is Valid`
      (`/Game/Blueprints/Component/BP_UIComponent.ToggleToolTip` _returnvalue true (`|FormatText` "Press [{KeyBinding}] to buy" (`/Game/Blueprints/HelperFunctions.GetInputActionKeyName` "Interact"))))))

(event `self.E OnPlayerExit`
  (params (Character :type "/Game/Blueprints/Character/BP_Base_Character Object Reference"))
  (bind _returnvalue (`self.GetComponentByClass` Character "/Game/Blueprints/Component/BP_UIComponent.BP_UIComponent_C"))
  (if (`Pawn.IsPlayerControlled` Character)
    (`/Engine/EditorBlueprintResources/StandardMacros.IsValid` _returnvalue
      (:`Is Valid`
        (`/Game/Blueprints/Component/BP_UIComponent.ToggleToolTip` _returnvalue false "")))))

(event `self.E Invoke`
  (params (Character :type "/Game/Blueprints/Character/BP_Base_Character Object Reference") (Inventory :type "/Game/Blueprints/Component/BP_Inventory Object Reference"))
  (if (>= (`/Game/Blueprints/Component/BP_Inventory.Cash` Inventory) (`self.Cost`))
    (`self.BuyItem` Inventory)))

(fn `BuyItem`
  (params (Inventory :type "/Game/Blueprints/Component/BP_Inventory Object Reference"))
  (bind _returnvalue (`|SpawnActorFromClass` (`self.Item Ref`) (`KismetMathLibrary.MakeTransform` (0.0 0.0 -1000.0)) "AlwaysSpawn" "OverrideRootScale" null null))
  (`/Game/Blueprints/Component/BP_Inventory.Add To Inventory` Inventory _returnvalue)
  (`/Game/Blueprints/Component/BP_Inventory.Add To Cash` Inventory (* (`self.Cost`) -1)))

(fn `UserConstructionScript`
  (`parent.UserConstructionScript`)
  (`ChildActorComponent.SetChildActorClass` (`self.ChildActor`) (`self.Item Ref`)))