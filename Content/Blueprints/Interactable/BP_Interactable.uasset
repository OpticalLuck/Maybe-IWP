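; BP_Interactable is a base actor for objects that characters interact with by entering a boundary box.
; Overlap events cast to BP_Base_Character and fire enter and exit hooks, with enter limited to players unless CanAIInteract is set, while exit fires for any character.
; The enter, exit and invoke events are empty here, and the construction script sizes the box from BoxExtent.
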(event `self.ReceiveActorBeginOverlap`
  (params (OtherActor :type "Actor Object Reference"))
  (bind _asbp_base_character (cast `/Game/Blueprints/Character/BP_Base_Character` OtherActor))
  (bind _returnvalue (`Pawn.IsPlayerControlled` _asbp_base_character))
  (if (or (and (`self.Can AI Interact`) (not _returnvalue)) _returnvalue)
    (`self.E OnPlayerEnter` _asbp_base_character)))

(event `self.ReceiveActorEndOverlap`
  (params (OtherActor :type "Actor Object Reference"))
  (bind _asbp_base_character (cast `/Game/Blueprints/Character/BP_Base_Character` OtherActor))
  (`self.E OnPlayerExit` _asbp_base_character))

(event `E OnPlayerEnter`
  (params (Character :type "/Game/Blueprints/Character/BP_Base_Character Object Reference")))

(event `E OnPlayerExit`
  (params (Character :type "/Game/Blueprints/Character/BP_Base_Character Object Reference")))

(event `E Invoke`
  (params (Character :type "/Game/Blueprints/Character/BP_Base_Character Object Reference") (Inventory :type "/Game/Blueprints/Component/BP_Inventory Object Reference")))

(fn `UserConstructionScript`
  (`BoxComponent.SetBoxExtent` (`self.BoundaryBox`) (`self.BoxExtent`) true))