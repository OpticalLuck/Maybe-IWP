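; BP_HealthDrop is a short-lived health pickup that heals the player character who enters it.
; On player enter, it calls HealPlayer on the character's BPCharacterInfo with HealAmount, plays a 2D sound, then destroys itself.
; BeginPlay starts a one-shot timer that destroys the drop after five seconds if it is not collected.
; The player exit and invoke events are left empty.
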(event `self.E OnPlayerEnter`
  (params (Character :type "/Game/Blueprints/Character/BP_Base_Character Object Reference"))
  (`/Game/Blueprints/Component/BP_CharacterInfo.Heal Player` (`/Game/Blueprints/Character/BP_Base_Character.BP_CharacterInfo` Character) (`self.Heal Amount`))
  (`GameplayStatics.PlaySound2D` (`self.Sound Cue`) 1.0 1.0 0.0 null null)
  (`self.K2_DestroyActor`))

(event `self.E OnPlayerExit`
  (params (Character :type "/Game/Blueprints/Character/BP_Base_Character Object Reference")))

(event `self.E Invoke`
  (params (Character :type "/Game/Blueprints/Character/BP_Base_Character Object Reference") (Inventory :type "/Game/Blueprints/Component/BP_Inventory Object Reference")))

(event `self.ReceiveBeginPlay`
  (`KismetSystemLibrary.K2_SetTimerDelegate` (delegate `Timer`) 5.0))

(event `Timer`
  (`self.K2_DestroyActor`))

(fn `UserConstructionScript`
  (`parent.UserConstructionScript`))